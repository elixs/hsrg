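; Melee lane minion character for the Dawn variant, handling how it reacts to hits from the hero's sword.
; Both blade collisions start disabled, and a capsule overlap with the hero sword counts only while the minion is vulnerable.
; A hit launches it along the player's forward vector, feeds damage and signed hit angle to its Anim Blueprint, and decrements hit points.
; It also widens pawn-sensing vision and grants brief invulnerability.
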(event OnComponentBeginOverlap(CapsuleComponent)
  (params (OverlappedComponent :type Primitive%20Component%20Object%20Reference) (OtherActor :type Actor%20Object%20Reference) (OtherComp :type Primitive%20Component%20Object%20Reference) (OtherBodyIndex :type Integer) (bFromSweep :type Boolean) (SweepResult :type Hit%20Result%20Structure%20%28by%20ref%29))
  (bind _returnvalue (Transformation|GetActorForwardVector))
  (bind _returnvalue_2 (Game|Player|GetPlayerPawn 0))
  (bind (_x _y) (Math|Vector|BreakVector _returnvalue))
  (bind _returnvalue_3 (Transformation|GetActorForwardVector _returnvalue_2))
  (bind (_x_2 _y_2) (Math|Vector|BreakVector _returnvalue_3))
  (Utilities|Casting|CastToBP_Blade_HeroSword11 OtherActor)
  (if (Variables|Default|GetVulnerable)
    (bind _asabp_minion_lane_melee_dawn (Utilities|Casting|CastToABP_Minion_Lane_Melee_Dawn (Components|SkeletalMesh|GetAnimInstance (Variables|Character|GetMesh))))
    (Variables|/Game/Blueprints/ABP_Minion_Lane_Melee_Dawn.ABP_Minion_Lane_Melee_Dawn_C|SetTakeDamage? _asabp_minion_lane_melee_dawn true)
    (Variables|Default|SetbIsHit true)
    (Character|LaunchCharacter (* _returnvalue_3 1e+03) false false)
    (bind _asabp_minion_lane_melee_dawn_2 (Utilities|Casting|CastToABP_Minion_Lane_Melee_Dawn (Components|SkeletalMesh|GetAnimInstance (Variables|Character|GetMesh))))
    (Variables|/Game/Blueprints/ABP_Minion_Lane_Melee_Dawn.ABP_Minion_Lane_Melee_Dawn_C|SetTakeDamage? _asabp_minion_lane_melee_dawn_2 true)
    (Variables|/Game/Blueprints/ABP_Minion_Lane_Melee_Dawn.ABP_Minion_Lane_Melee_Dawn_C|SetHitDirection _asabp_minion_lane_melee_dawn_2 (Class|KismetMathLibrary|DegAtan2 (- (* _x_2 _y) (* _y_2 _x)) (+ (* _x_2 _x) (* _y_2 _y))))
    (Variables|Default|SetHitPoints (- (Variables|Default|GetHitPoints) 1))
    (Class|PawnSensingComponent|SetPeripheralVisionAngle (Variables|Default|GetPawnSensor) 1.8e+02)
    (Variables|Default|SetVulnerable false)
    (Utilities|FlowControl|Delay 0.5)
    (Variables|Default|SetVulnerable true)))

(event EventBeginPlay
  (Collision|SetCollisionEnabled (Variables|Default|GetLeftBlade) "NoCollision")
  (Collision|SetCollisionEnabled (Variables|Default|GetRightBlase) "NoCollision"))

(event EventTick
  (params (DeltaSeconds :type Float%20%28single-precision%29)))

(fn ConstructionScript)